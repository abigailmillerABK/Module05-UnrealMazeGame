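; Destroyable actor that removes itself when the player slashes it with an axe while inside its Collision component.
; Overlap events toggle an IsCollided flag, which any actor sets on entering but only a CustomPlayerCharacter clears on leaving.
; Tick polls that flag and the AxeSlash state of the last overlapping actor, cast to CustomPlayerCharacter, and destroys the actor when both are true.
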(event `self.ReceiveBeginPlay`
  (set `self.isCollided` false))

(event `self.ReceiveTick`
  (params (DeltaSeconds :type "Float (single-precision)"))
  (bind _ascustom_player_character (cast `/Game/CustomContent/Player/CustomPlayerCharacter` (stale `self.Collision.OnComponentBeginOverlap` OtherActor)))
  (if (and (`/Game/CustomContent/Player/CustomPlayerCharacter.AxeSlash` _ascustom_player_character) (`self.isCollided`))
    (`self.K2_DestroyActor`)))

(event `self.Collision.OnComponentBeginOverlap`
  (params (OverlappedComponent :type "PrimitiveComponent Object Reference") (OtherActor :type "Actor Object Reference") (OtherComp :type "PrimitiveComponent Object Reference") (OtherBodyIndex :type Integer) (bFromSweep :type Boolean) (SweepResult :type "HitResult Structure (by ref)"))
  (set `self.isCollided` true))

(event `self.Collision.OnComponentEndOverlap`
  (params (OverlappedComponent :type "PrimitiveComponent Object Reference") (OtherActor :type "Actor Object Reference") (OtherComp :type "PrimitiveComponent Object Reference") (OtherBodyIndex :type Integer))
  (cast `/Game/CustomContent/Player/CustomPlayerCharacter` OtherActor)
  (set `self.isCollided` false))

(fn `UserConstructionScript`)